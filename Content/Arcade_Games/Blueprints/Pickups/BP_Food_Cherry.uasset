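; Cherry bonus pickup for an arcade game that awards points when the player eats it.
; On BeginPlay it plays a spawn particle effect and sound.
; When BP_Player overlaps its collision, it plays eat effects, destroys its visual and collision components, spawns a 500-score popup actor, and destroys itself after a delay.
; The overlap also adds CherryPts to the game instance and runs its extra-life check.
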(event OnComponentBeginOverlap(Collision)
  (params (OverlappedComponent :type Primitive%20Component%20Object%20Reference) (OtherActor :type Actor%20Object%20Reference) (OtherComp :type Primitive%20Component%20Object%20Reference) (OtherBodyIndex :type Integer) (bFromSweep :type Boolean) (SweepResult :type Hit%20Result%20Structure%20%28by%20ref%29))
  (Utilities|Casting|CastToBP_Player OtherActor)
  (Utilities|FlowControl|Sequence
    (:then_0
      ;[0 1 0 1 50] Fryit Cherry Eaten Handing
      (Audio|PlaySound2D "/Game/Arcade_Games/Audio/Cue/SC_Eat_Spacial.SC_Eat_Spacial" 1.0 1.0 0.0 0 0)
      (Components|Activation|Activate (Variables|Default|GetVFX_Eaten) false)
      (Components|DestroyComponent (Variables|Default|GetSM_Cherry_01))
      (Game|SpawnActorfromClass "/Game/Arcade_Games/Blueprints/Misc/BP_Score_500.BP_Score_500_C" (Math|Transform|MakeTransform (Transformation|GetWorldLocation (Variables|Default|GetDefaultSceneRoot)) "0, 0, 0" "1.000000,1.000000,1.000000") "Undefined" "MultiplyWithRoot" 0 0)
      (Utilities|FlowControl|Delay 5.0)
      (Actor|DestroyActor))
    (:then_1
      ;[0 1 0 1 50] Increment Score
      (bind _asbp_game_instance (Utilities|Casting|CastToBP_GameInstance (Game|GetGameInstance)))
      (Default|AddPoints _asbp_game_instance (Variables|Default|GetCherryPts))
      (Default|1upCHECK _asbp_game_instance))))

(event EventBeginPlay
  (CallFunction|SpawnFX) ; Goodie Spawn FX
)

(fn ConstructionScript)

(fn SpawnFX
  (bind _returnvalue (Effects|SpawnEmitteratLocation "/Game/Arcade_Games/VFX/P_levelUp.P_levelUp" (Transformation|GetWorldLocation (Variables|Default|GetCollision))))
  (Transformation|SetWorldScale3D _returnvalue "3.000000,3.000000,3.000000")
  (Audio|PlaySound2D "/Game/Arcade_Games/Audio/Cue/SC_Fruit_Spawn.SC_Fruit_Spawn" 1.0 1.0 0.0 0 0))