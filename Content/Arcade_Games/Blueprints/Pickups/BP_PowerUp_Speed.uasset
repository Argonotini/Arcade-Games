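; BP_PowerUp_Speed is an arcade pickup that gives the player a speed boost when eaten.
; On BeginPlay it spawns a scaled level-up particle effect and a spawn sound at its collision location.
; When BP_Player overlaps it, it calls SpeedBoost on the player, plays eat audio and VFX, and removes its collision, mesh and glow.
; It then stops rotating and destroys itself after a short delay.
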(event OnComponentBeginOverlap(Collision)
  (params (OverlappedComponent :type Primitive%20Component%20Object%20Reference) (OtherActor :type Actor%20Object%20Reference) (OtherComp :type Primitive%20Component%20Object%20Reference) (OtherBodyIndex :type Integer) (bFromSweep :type Boolean) (SweepResult :type Hit%20Result%20Structure%20%28by%20ref%29))
  ;[0 1 0 1 50] Power - Up Eaten
  (bind _asbp_player (Utilities|Casting|CastToBP_Player OtherActor))
  (Default|SpeedBoost _asbp_player)
  (Audio|PlaySound2D "/Game/Arcade_Games/Audio/Cue/SC_Eat_Spacial.SC_Eat_Spacial" 1.0 1.0 0.0 0 0)
  (Components|Activation|Activate (Variables|Default|GetVFX_Eaten) false)
  (Components|DestroyComponent (Variables|Default|GetCollision))
  (Variables|/Script/Engine.RotatingMovementComponent|SetRotationRate (Variables|Default|GetRotatingMovement) "0, 0, 0")
  (Utilities|FlowControl|Delay 5.0)
  (Actor|DestroyActor))

(event EventBeginPlay
  (CallFunction|SpawnFX) ; Goodie Spawn FX
)

(fn ConstructionScript)

(fn SpawnFX
  (bind _returnvalue (Effects|SpawnEmitteratLocation "/Game/Arcade_Games/VFX/P_levelUp.P_levelUp" (Transformation|GetWorldLocation (Variables|Default|GetCollision))))
  (Transformation|SetWorldScale3D _returnvalue "3.000000,3.000000,3.000000")
  (Audio|PlaySound2D "/Game/Arcade_Games/Audio/Cue/SC_Fruit_Spawn.SC_Fruit_Spawn" 1.0 1.0 0.0 0 0))