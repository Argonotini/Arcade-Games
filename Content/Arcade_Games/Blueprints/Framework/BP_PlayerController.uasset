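; Player controller for the arcade games project that handles global hotkeys for pausing, quitting, game speed and debug display.
; Pause flip-flops the paused state and the WB_PauseMenu widget, while mutually exclusive Slow and Fast toggles set global time dilation.
; Debug input toggles collision and navigation views through console commands.
; BPI_Get_DebugInfo exposes the HUD, speed and debug flags; the HUD key only flips its flag here.
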(event Input|ActionEvents|InputActionPause
  (params (Key :type Key%20Structure :default "None"))
  ;[0 1 0] Pause Game
  (:Pressed
    (Utilities|FlowControl|FlipFlop
      (:A
        (Game|SetGamePaused true)
        (bind _returnvalue (UserInterface|CreateWidget "/Game/Arcade_Games/UMG/WB_PauseMenu.WB_PauseMenu_C"))
        (bind _output_get (Variables|Default|SetPauseMenu _returnvalue))
        (UserInterface|Viewport|AddtoViewport _output_get 0))
      (:B
        (Game|SetGamePaused false)
        (Widget|RemovefromParent (Variables|Default|GetPauseMenu))))))

(event Input|ActionEvents|InputActionShowDebug
  (params (Key :type Key%20Structure :default "None"))
  (bind _returnvalue (Game|GetPlayerController 0))
  ;[1 0 0.6284] Show Debug: Collision / MeshBound
  (:Pressed
    (bind _output_get (Variables|Debug|SetbShowDebug? (not (Variables|Debug|GetbShowDebug?))))
    (if _output_get
      (Development|ExecuteConsoleCommand "show collision" _returnvalue)
      (Development|ExecuteConsoleCommand "ShowFlag.Navigation = 1" 0)
      (Development|ExecuteConsoleCommand "show navigation" _returnvalue)
      (else
        (Development|ExecuteConsoleCommand "show collision" _returnvalue)
        (Development|ExecuteConsoleCommand "ShowFlag.Navigation = 0" _returnvalue)))))

(event Input|ActionEvents|InputActionSlow
  (params (Key :type Key%20Structure :default "None"))
  ;[1 0 0.6284] Slowing down the game (1x-0.15x)
  (:Pressed
    (bind _output_get (Variables|Debug|SetbSlomo? (not (Variables|Debug|GetbSlomo?))))
    (if _output_get
      (bind _output_get_2 (Variables|Debug|SetbFast? false))
      (if (not _output_get_2)
        (Utilities|Time|SetGlobalTimeDilation 0.15))
      (else
        (bind _output_get_3 (Variables|Debug|SetbFast? false))
        (if (not _output_get_3)
          (Utilities|Time|SetGlobalTimeDilation 1.0))))))

(event Input|ActionEvents|InputActionFast
  (params (Key :type Key%20Structure :default "None"))
  ;[1 0 0.6284] Fast down the game (1x-2x)
  (:Pressed
    (bind _output_get (Variables|Debug|SetbFast? (not (Variables|Debug|GetbFast?))))
    (if _output_get
      (bind _output_get_2 (Variables|Debug|SetbSlomo? false))
      (if (not _output_get_2)
        (Utilities|Time|SetGlobalTimeDilation 2.0))
      (else
        (bind _output_get_3 (Variables|Debug|SetbSlomo? false))
        (if (not _output_get_3)
          (Utilities|Time|SetGlobalTimeDilation 1.0))))))

(event Input|ActionEvents|InputActionShowHUD
  (params (Key :type Key%20Structure :default "None"))
  ;[1 0 0.6284] Show Debug HUD
  (:Pressed
    (Variables|Debug|SetbShowHUD? (not (Variables|Debug|GetbShowHUD?)))))

(event Input|ActionEvents|InputActionExitGame
  (params (Key :type Key%20Structure :default "None"))
  ;[1 0 0.6284] Exit Game
  (:Pressed
    (Game|QuitGame 0 "Quit" false)))

(fn ConstructionScript)

(fn BPIGetDebugInfo
  (return (Variables|Debug|GetbShowHUD?) (Variables|Debug|GetbSlomo?) (Variables|Debug|GetbFast?) (Variables|Debug|GetbShowDebug?)))